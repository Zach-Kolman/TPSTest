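; Base AI character Blueprint that handles health, damage and a melee weapon carried on the back or in hand.
; On BeginPlay it fills health, links itself to its widget HUD, then spawns the default weapon onto the back socket.
; Headshots zero health, while other hits flag the enemy as found and body hits subtract damage.
; Equip/Unequip flip-flops the weapon between sword and back sockets; EnableCombat plays the equip montage.
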(event Custom|SpawnDefaultWeapon
  (bind _returnvalue (Game|SpawnActorfromClass (Variables|Default|GetWeaponClass) (Transformation|GetWorldTransform (Variables|Default|GetSphere)) "Undefined" 0 0))
  (bind _output_get (Variables|Default|SetWeapon_BP _returnvalue))
  (Transformation|AttachComponentToComponent _output_get (Variables|Character|GetMesh) "BackSocket" "KeepWorld" "KeepWorld" "KeepWorld" true)
  (Default|DestorySPhere _output_get))

(event Custom|Equip/Unequip
  (Utilities|FlowControl|FlipFlop
    (:A
      (Transformation|AttachComponentToComponent (Variables|Default|GetWeapon_BP) (Variables|Character|GetMesh) "SwordSocket" "SnapToTarget" "SnapToTarget" "SnapToTarget" true)
      (Variables|Default|SetEquipWeapon true))
    (:B
      (Transformation|AttachComponentToComponent (Variables|Default|GetWeapon_BP) (Variables|Character|GetMesh) "BackSocket" "KeepWorld" "KeepWorld" "KeepWorld" true)
      (Variables|Default|SetEquipWeapon false))))

(event Custom|EnableCombat
  (Animation|PlayAnimMontage "/Game/AI_Bleuprint/Montages/newEquipMontageAI.newEquipMontageAI" 1.0 "None")
  (Development|PrintString "it also worked"))

(event EventBeginPlay
  (Variables|Default|SetCurrentHealth (Variables|Default|GetMaxHealth))
  (bind _asaihud (Utilities|Casting|CastToAIHud (UserInterface|GetUserWidgetObject (Variables|Default|GetAIWidget))))
  (Variables|/Game/AI_Bleuprint/AIHud.AIHud_C|SetOwner _asaihud self)
  (CallFunction|SpawnDefaultWeapon))

(event EventITakeDamage
  (params (CollName :type Box%20Component%20Object%20Reference) (Damage :type Float%20%28single-precision%29))
  (if (== CollName (Variables|Default|GetHeadshotCollision))
    (Variables|Default|SetCurrentHealth 0.0)
    (else
      (Variables|Default|SetEnemyFound true)
      (if (== CollName (Variables|Default|GetBodyCollision))
        (Variables|Default|SetCurrentHealth (- (Variables|Default|GetCurrentHealth) Damage))))))

(fn ConstructionScript)